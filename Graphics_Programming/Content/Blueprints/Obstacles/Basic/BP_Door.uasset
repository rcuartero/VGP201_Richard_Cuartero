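; BP_Door is an obstacle door that moves its wall vertically when an attached switch notifies it.
; On BeginPlay it binds to the switch's notify event in an observer pattern, if a switch is set.
; The first notification plays a timeline that scales the wall's relative Z offset by the actor's bounds height.
; The moving flag is never reset, so later notifications are ignored.
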(event Custom|Platform%20Notified
  ;[1 1 1] Set Up Observer
  ;[1 1 1] Start Moving Platform
  (if (not (Variables|Default|GetisMoving))
    (Variables|Default|SetisMoving true)
    (bind _move_timer (Timeline|Move%20Platform Play)
      (:Update
        (Transformation|SetRelativeLocation (Variables|Default|GetWall) (Math|Vector|MakeVector 0.0 0.0 (* _move_timer (* (.z (.BoxExtent (Collision|GetActorBounds self false false))) 1.8))) false false)))))

(event EventBeginPlay
  (bind _attachedswitch (Variables|Default|GetattachedSwitch))
  (Variables|Default|SetstartPos (Transformation|GetActorLocation))
  ;[1 1 1] Set Up Observer
  (if (Utilities|IsValid _attachedswitch)
    (EventDispatchers|BindEventtoNotify _attachedswitch (delegate Custom|Platform%20Notified))))

(event Collision|EventActorBeginOverlap
  (params (OtherActor :type Actor%20Object%20Reference)))

(event EventTick
  (params (DeltaSeconds :type Float%20%28single-precision%29)))

(fn ConstructionScript)