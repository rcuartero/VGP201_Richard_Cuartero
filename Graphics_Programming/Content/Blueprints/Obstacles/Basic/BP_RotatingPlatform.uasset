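; BP_RotatingPlatform is an obstacle platform that rotates by a set yaw step each time its attached switch notifies it.
; On BeginPlay it registers PlatformNotified with the switch as an observer, if one is assigned.
; A timeline drives the relative yaw from the stored reference angle, ignoring notifications while moving.
; On finish it adds the step to that reference, so successive rotations accumulate.
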(event Custom|Platform%20Notified
  (bind _rotatevalue (Variables|Default|GetrotateValue))
  ;[1 1 1] Set Up Observer
  ;[1 1 1] Start Moving Platform
  (if (not (Variables|Default|GetisMoving))
    (Variables|Default|SetisMoving true)
    (bind _rotate_timer (Timeline|Rotate%20Timeline PlayFromStart)
      (:Update
        (Transformation|SetActorRelativeRotation (Math|Rotator|MakeRotator 0.0 0.0 (+ (* _rotate_timer _rotatevalue) (Variables|Default|GetrotateRef)))))
      (:Finished
        (Variables|Default|SetisMoving false)
        (Variables|Default|SetrotateRef (+ (Variables|Default|GetrotateRef) _rotatevalue))))))

(event EventBeginPlay
  (bind _attachedswitch (Variables|Default|GetattachedSwitch))
  ;[1 1 1] Set Up Observer
  (if (Utilities|IsValid _attachedswitch)
    (EventDispatchers|BindEventtoNotify _attachedswitch (delegate Custom|Platform%20Notified))))

(event Collision|EventActorBeginOverlap
  (params (OtherActor :type Actor%20Object%20Reference)))

(event EventTick
  (params (DeltaSeconds :type Float%20%28single-precision%29)))

(fn ConstructionScript)