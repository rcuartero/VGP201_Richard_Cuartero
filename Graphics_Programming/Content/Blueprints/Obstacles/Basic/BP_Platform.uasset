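; BP_Platform is an obstacle platform that starts moving when its attached switch notifies it.
; On BeginPlay it registers as an observer of that switch, and an IsMoving flag, never reset here, lets only the first notification start the MovePlatform timeline.
; Each timeline update adds EndPos scaled by MoveTimer to the current actor location and sets it as relative location without sweep, so the offset accumulates per update.
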(event Custom|Platform%20Notified
  ;[1 1 1] Set Up Observer
  ;[1 1 1] Start Moving Platform
  (if (not (Variables|Default|GetisMoving))
    (Variables|Default|SetisMoving true)
    (bind _move_timer (Timeline|Move%20Platform Play)
      (:Update
        (Transformation|SetActorRelativeLocation (+ (Transformation|GetActorLocation) (* _move_timer (Variables|Default|GetendPos))))))))

(event EventBeginPlay
  (bind _attachedswitch (Variables|Default|GetattachedSwitch))
  ;[1 1 1] Set Up Observer
  (if (Utilities|IsValid _attachedswitch)
    (EventDispatchers|BindEventtoNotify _attachedswitch (delegate Custom|Platform%20Notified))))

(event Collision|EventActorBeginOverlap
  (params (OtherActor :type Actor%20Object%20Reference)))

(event EventTick
  (params (DeltaSeconds :type Float%20%28single-precision%29)))

(fn ConstructionScript)