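; BP_Switch is a switch obstacle that activates attached obstacles through CallNotify when hit by a projectile or used by the player.
; A BP_Projectile overlap fires it immediately.
; A BP_Player overlap binds the player's interact event and arms CanInteract, and leaving unbinds it.
; Interacting fires once and clears CanInteract, so the player must re-enter to use it again, while projectiles ignore that flag.
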(event Custom|Interacting%20with%20Player
  ;[1 1 1] Activate obstacles attached
  ;;[1 1 1] Activated when player in range
  (if (Variables|Default|GetcanInteract)
    (Default|CallNotify)
    (Variables|Default|SetcanInteract false)
    (else
      (Development|PrintString "Can't Interact"))))

(event EventBeginPlay)

(event EventTick
  (params (DeltaSeconds :type Float%20%28single-precision%29)))

(event Collision|EventActorBeginOverlap
  (params (OtherActor :type Actor%20Object%20Reference))
  ;[1 1 1] Activate obstacles attached
  ;;[1 1 1] Activated when projectile hits
  (Utilities|Casting|CastToBP_Projectile OtherActor
    (:then
      (Default|CallNotify))
    (:CastFailed
      ;;[1 1 1] Activated when player in range
      (bind _asbp_player (Utilities|Casting|CastToBP_Player OtherActor))
      (EventDispatchers|BindEventtoInteract _asbp_player (delegate Custom|Interacting%20with%20Player))
      (Variables|Default|SetcanInteract true))))

(event Collision|EventActorEndOverlap
  (params (OtherActor :type Actor%20Object%20Reference))
  ;[1 1 1] Activate obstacles attached
  ;;[1 1 1] Activated when player in range
  (bind _asbp_player (Utilities|Casting|CastToBP_Player OtherActor))
  (EventDispatchers|UnbindEventfromInteract _asbp_player (delegate Custom|Interacting%20with%20Player)))

(fn ConstructionScript)