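; BP_Player is the player character, with Enhanced Input movement, look, jump, interact and an aim-and-shoot mechanic that hands control to the projectile.
; Aiming requires CanAim and a downward ground trace at its start, and suspends movement input while held.
; Shooting spawns BP_Projectile at AttackPoint facing the camera, passes it a player reference and possesses it.
; Player input is disabled on firing, then restored with aim cleared upon repossession.
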(event Input|EnhancedActionEvents|EnhancedInputActionINPUT_Shoot
  (params (ActionValue :type Boolean) (ElapsedSeconds :type Float%20%28double-precision%29) (TriggeredSeconds :type Float%20%28double-precision%29) (InputAction :type Input%20Action%20Object%20Reference :default "/Game/Blueprints/Player/Player/Input/INPUT_Shoot.INPUT_Shoot"))
  ;[1 1 1] Aim/Shoot
  (if (Variables|Default|GetisAiming)
    (Input|DisableInput 0)
    (bind _returnvalue (Game|SpawnActorfromClass "/Game/Blueprints/Player/Projectile/BP_Projectile.BP_Projectile_C" (Transformation|GetWorldTransform (Variables|Default|GetAttackPoint)) "AlwaysSpawn" "MultiplyWithRoot" 0 0))
    (Transformation|SetRelativeRotation (Variables|/Script/Engine.Actor|GetRootComponent _returnvalue) (Transformation|GetWorldRotation (Variables|Components|GetCamera)) false false)
    (Variables|/Game/Blueprints/Player/Projectile/BP_Projectile.BP_Projectile_C|Setplayer _returnvalue self)
    (Pawn|Possess (Game|GetPlayerController 0) _returnvalue)
    (Audio|PlaySound2D "/Game/Audio/SFX/mixkit-air-woosh-1489.mixkit-air-woosh-1489" 1.0 1.0 0.0 0 0)))

(event Input|EnhancedActionEvents|EnhancedInputActionINPUT_Movement
  (params (ActionValue :type Vector%202D%20Structure) (ElapsedSeconds :type Float%20%28double-precision%29) (TriggeredSeconds :type Float%20%28double-precision%29) (InputAction :type Input%20Action%20Object%20Reference :default "/Game/Blueprints/Player/Player/Input/INPUT_Movement.INPUT_Movement"))
  (bind _camera (Variables|Components|GetCamera))
  ;[1 1 1] Movement
  (if (not (Variables|Default|GetisAiming))
    (Pawn|Input|AddMovementInput (Math|Vector|GetRightVector _camera) (.x ActionValue) false)
    (Pawn|Input|AddMovementInput (Math|Vector|GetForwardVector _camera) (.y ActionValue) false)))

(event Input|EnhancedActionEvents|EnhancedInputActionINPUT_Look
  (params (ActionValue :type Vector%202D%20Structure) (ElapsedSeconds :type Float%20%28double-precision%29) (TriggeredSeconds :type Float%20%28double-precision%29) (InputAction :type Input%20Action%20Object%20Reference :default "/Game/Blueprints/Player/Player/Input/INPUT_Look.INPUT_Look"))
  ;[1 1 1] Look around
  (Pawn|Input|AddControllerYawInput (.x ActionValue))
  (bind _result (Math|Float|NegateFloat (.y ActionValue))
    (:%20%20
      (Pawn|Input|AddControllerPitchInput _result))))

(event Input|EnhancedActionEvents|EnhancedInputActionINPUT_Jump
  (params (ActionValue :type Boolean) (ElapsedSeconds :type Float%20%28double-precision%29) (TriggeredSeconds :type Float%20%28double-precision%29) (InputAction :type Input%20Action%20Object%20Reference :default "/Game/Blueprints/Player/Player/Input/INPUT_Jump.INPUT_Jump"))
  ;[1 1 1] Movement
  (Character|Jump))

(event Input|EnhancedActionEvents|EnhancedInputActionINPUT_AIM
  (params (ActionValue :type Boolean) (ElapsedSeconds :type Float%20%28double-precision%29) (TriggeredSeconds :type Float%20%28double-precision%29) (InputAction :type Input%20Action%20Object%20Reference :default "/Game/Blueprints/Player/Player/Input/INPUT_AIM.INPUT_AIM"))
  (bind _capsulecomponent (Variables|Collision|GetCapsuleComponent))
  (bind _returnvalue (Transformation|GetWorldLocation _capsulecomponent))
  ;[1 1 1] Aim/Shoot
  (:Started
    (if (Variables|Default|GetcanAim)
      ;;[1 1 1] Ground Check
      (bind _returnvalue_2 (Collision|LineTraceByChannel _returnvalue (+ _returnvalue (* (Math|Vector|VectorDown) (Variables|Default|GetgroundCheckRange))) "TraceTypeQuery1" false 0 "ForDuration" true "(R=1.000000,G=0.000000,B=0.000000,A=1.000000)" "(R=0.000000,G=1.000000,B=0.000000,A=1.000000)" 2.0))
      (if _returnvalue_2
        (Variables|Default|SetisAiming true))))
  (:Completed
    (Variables|Default|SetisAiming false)))

(event Input|EnhancedActionEvents|EnhancedInputActionINPUT_Interact
  (params (ActionValue :type Boolean) (ElapsedSeconds :type Float%20%28double-precision%29) (TriggeredSeconds :type Float%20%28double-precision%29) (InputAction :type Input%20Action%20Object%20Reference :default "/Game/Blueprints/Player/Player/Input/INPUT_Interact.INPUT_Interact"))
  ;[1 1 1] Interact
  (:Started
    (Default|CallInteract)))

(event EventBeginPlay
  (bind _returnvalue (Game|GetPlayerController 0))
  (bind _returnvalue_2 (PlayerController|LocalPlayerSubsystems|GetEnhancedInputLocalPlayerSubsystem _returnvalue))
  (Utilities|IsValid _returnvalue_2
    (:Is%20Valid
      (Input|AddMappingContext _returnvalue_2 "/Game/Blueprints/Player/Player/Input/INPUT_ContextMap.INPUT_ContextMap" 0 "(bIgnoreAllPressedKeysUntilRelease=True,bForceImmediately=False,bNotifyUserSettings=False)"))))

(event Collision|EventActorBeginOverlap
  (params (OtherActor :type Actor%20Object%20Reference)))

(event EventTick
  (params (DeltaSeconds :type Float%20%28single-precision%29)))

(event EventPossessed
  (params (NewController :type Controller%20Object%20Reference))
  ;[1 1 1] Reset after repossessing
  (CallFunction|ResetState))

(fn ConstructionScript)

(fn ResetState
  (Variables|Default|SetisAiming false)
  (Input|EnableInput 0))

(fn SetCanAim
  (params (value :type Boolean))
  (Variables|Default|SetcanAim value))