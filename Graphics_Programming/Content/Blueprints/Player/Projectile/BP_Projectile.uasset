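; BP_Projectile is a player-steered projectile pawn that serves as a teleport swap mechanic.
; It flies continuously along its camera's forward vector through FloatingPawnMovement, while look input rotates the actor.
; Swap input moves the stored Player to the projectile's location and yaw.
; Swapping, or overlapping anything but another projectile, calls DisableProjectile, which re-possesses the Player and destroys the projectile.
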(event OnComponentBeginOverlap(SphereCollider)
  (params (OverlappedComponent :type Primitive%20Component%20Object%20Reference) (OtherActor :type Actor%20Object%20Reference) (OtherComp :type Primitive%20Component%20Object%20Reference) (OtherBodyIndex :type Integer) (bFromSweep :type Boolean) (SweepResult :type Hit%20Result%20Structure%20%28by%20ref%29))
  ;[1 1 1] Handle Collision
  (Utilities|Casting|CastToBP_Projectile OtherActor
    (:CastFailed
      (Components|Activation|SetActive (Variables|Default|GetFloatingPawnMovement) false false)
      (CallFunction|DisableProjectile))))

(event Input|EnhancedActionEvents|EnhancedInputActionINPUT_Swap
  (params (ActionValue :type Boolean) (ElapsedSeconds :type Float%20%28double-precision%29) (TriggeredSeconds :type Float%20%28double-precision%29) (InputAction :type Input%20Action%20Object%20Reference :default "/Game/Blueprints/Player/Player/Input/INPUT_Swap.INPUT_Swap"))
  ;[1 1 1] Swap Mechanic
  (Transformation|SetActorLocationAndRotation (Variables|Default|Getplayer) (Transformation|GetActorLocation) (Math|Rotator|MakeRotator 0.0 0.0 (.yaw (Transformation|GetActorRotation))))
  (CallFunction|DisableProjectile))

(event Input|EnhancedActionEvents|EnhancedInputActionINPUT_Look
  (params (ActionValue :type Vector%202D%20Structure) (ElapsedSeconds :type Float%20%28double-precision%29) (TriggeredSeconds :type Float%20%28double-precision%29) (InputAction :type Input%20Action%20Object%20Reference :default "/Game/Blueprints/Player/Player/Input/INPUT_Look.INPUT_Look"))
  ;[1 1 1] Changes projectile mesh rotation to match camera
  (Transformation|AddActorLocalRotation (Math|Rotator|MakeRotator 0.0 (.y ActionValue) (.x ActionValue)) false false))

(event EventTick
  (params (DeltaSeconds :type Float%20%28single-precision%29))
  ;[1 1 1] Projectile movement forward relative to Camera
  (Class|PawnMovementComponent|AddInputVector (Variables|Default|GetFloatingPawnMovement) (* (Math|Vector|GetForwardVector (Variables|Default|GetCamera)) (Variables|Default|GetSpeed)) false))

(fn ConstructionScript)

(fn DisableProjectile
  (Pawn|Possess (Game|GetPlayerController 0) (Variables|Default|Getplayer))
  (Actor|DestroyActor))